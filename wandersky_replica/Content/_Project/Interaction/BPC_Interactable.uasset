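; Actor component that makes its owner interactable, registering with an overlapping actor's BPC_Interactor on begin overlap and unregistering on end overlap.
; The interactor drives its active state and input events, completing instantly or after a hold time with normalized progress, and resetting on cancel or deactivation.
; Dispatchers broadcast active status, progress, completion and destruction.
; A tick after BeginPlay, it sets itself as the observed interactable on the owner's WBP_InteractionPrompt widget.
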(event Custom|OwnerStartOverlap
  (params (OverlappedActor :type Actor%20Object%20Reference) (OtherActor :type Actor%20Object%20Reference))
  ;[1 1 1] Overlap event callbacks
  (Development|PrintString "Start Overlap")
  (Default|AddInteractable (Actor|GetComponentbyClass OtherActor "/Game/_Project/Interaction/BPC_Interactor.BPC_Interactor_C") self))

(event Custom|OwnerEndOverlap
  (params (OverlappedActor :type Actor%20Object%20Reference) (OtherActor :type Actor%20Object%20Reference))
  ;[1 1 1] Overlap event callbacks
  (Default|RemoveInteractable (Actor|GetComponentbyClass OtherActor "/Game/_Project/Interaction/BPC_Interactor.BPC_Interactor_C") self)
  (Development|PrintString "Emd Overlap"))

(event Custom|SetAsActiveInteractable
  (params (Active :type Boolean))
  (Default|CallChangeActiveStatus Active)
  (if (not Active)
    (CallFunction|Reset)))

(event EventEndPlay
  (params (EndPlayReason :type EEndPlayReason%20Enum :default "Destroyed"))
  (Default|CallInteractableDestroyed self))

(event EventBeginPlay
  (CallFunction|BindtoOwnerOverlapEvents)
  (Utilities|FlowControl|DelayUntilNextTick)
  (CallFunction|SetSelfasInteractionPromptTarget))

(event Custom|OnInteractionStarted
  ;[1 1 1] Called by Interactor
  (if (CallFunction|HasProgress)
    (Variables|Default|SetIs%20Interacting true)
    (else
      (Default|CallInteractionComplete))))

(event Custom|OnInteractionOngoing
  (params (Elapsed :type Float%20%28double-precision%29))
  ;[1 1 1] Called by Interactor
  (if (Variables|Default|GetIs%20Interacting)
    (if (>= Elapsed (Variables|Default|GetHold%20Time))
      (CallFunction|Reset)
      (Default|CallInteractionComplete)
      (else
        (Default|CallInteractionProgress (Math|Float|SafeDivide Elapsed (Variables|Default|GetHold%20Time)))))))

(event Custom|OnInteractionCanceled
  ;[1 1 1] Called by Interactor
  (CallFunction|Reset))

(fn Reset
  (Variables|Default|SetIs%20Interacting false)
  (Default|CallInteractionProgress 0.0))

(fn HasProgress
  (return (> (Variables|Default|GetHold%20Time) 0.0)))

(fn BindtoOwnerOverlapEvents
  (bind _returnvalue (Components|GetOwner))
  (Collision|BindEventtoOnActorBeginOverlap _returnvalue (EventDispatchers|CreateEvent :!event Custom|OwnerStartOverlap))
  (Collision|BindEventtoOnActorEndOverlap _returnvalue (EventDispatchers|CreateEvent :!event Custom|OwnerEndOverlap)))

(fn SetSelfasInteractionPromptTarget
  (bind _returnvalue (Components|GetOwner))
  (bind _returnvalue_2 (Actor|GetComponentbyClass _returnvalue "/Script/UMG.WidgetComponent"))
  ;[1 1 1] Change to get components + find the right widget
  (Utilities|IsValid _returnvalue_2
    (:Is%20Valid
      (bind _aswbp_interaction_prompt (Utilities|Casting|CastToWBP_InteractionPrompt (UserInterface|GetWidget _returnvalue_2))
        (:then
          (Default|SetObservedInteractable _aswbp_interaction_prompt self))
        (:CastFailed
          (Development|PrintString (Utilities|String|Append (Utilities|GetDisplayName _returnvalue) " does not contain an Interaction Prompt") true true "(R=1.000000,G=0.113275,B=0.000000,A=1.000000)" 1e+01 :!label _label))))
    (:Is%20Not%20Valid
      (goto _label))))