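; Interactor component that tracks interactables in range and routes the owner's IA_Interact input to the active one.
; Add and remove functions maintain the list, bind or unbind each item's destroyed event, and re-pick the active interactable, notifying old and new on change.
; Tick re-selects the one closest to the owner, switched on only while several are in range, and selection stays locked during an interaction.
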(event Custom|StartPeriodicChecks
  (Components|Tick|SetComponentTickEnabled true))

(event Custom|EndPeriodicChecks
  (Components|Tick|SetComponentTickEnabled false))

(event Input|EnhancedActionEvents|EnhancedInputActionIA_Interact
  (params (ActionValue :type Boolean) (ElapsedSeconds :type Float%20%28double-precision%29) (TriggeredSeconds :type Float%20%28double-precision%29) (InputAction :type Input%20Action%20Object%20Reference :default "/Game/ThirdPerson/Input/Actions/IA_Interact.IA_Interact"))
  (:Started
    (bind _activeinteractable (Variables|Default|GetActiveInteractable)
      (:then
        (Variables|Default|SetIsInteracting true)
        (Default|OnInteractionStarted _activeinteractable))
      (:else)))
  (:Ongoing
    (bind _activeinteractable_2 (Variables|Default|GetActiveInteractable)
      (:then
        (Default|OnInteractionOngoing _activeinteractable_2 ElapsedSeconds))
      (:else)))
  (:Canceled
    (Variables|Default|SetIsInteracting false)
    (bind _activeinteractable_3 (Variables|Default|GetActiveInteractable)
      (:then
        (Default|OnInteractionCanceled _activeinteractable_3))
      (:else))))

(event EventTick
  (params (DeltaSeconds :type Float%20%28single-precision%29))
  (CallFunction|ChooseActiveInteractable))

(fn AddInteractable
  (params (NewItem :type BPC%20Interactable%20Object%20Reference%20%28by%20ref%29))
  (bind _interactablesinrange (Variables|Default|GetInteractablesInRange))
  (Utilities|Array|AddUnique _interactablesinrange NewItem)
  (Utilities|FlowControl|Sequence
    (:then_0
      (if (== (Utilities|Array|Length _interactablesinrange) 2)
        (CallFunction|StartPeriodicChecks)))
    (:then_1
      (if (not (Variables|Default|GetIsInteracting))
        (CallFunction|ChooseActiveInteractable)))
    (:then_2
      (EventDispatchers|BindEventtoInteractableDestroyed NewItem (EventDispatchers|CreateEvent :!event RemoveInteractable)))))

(fn RemoveInteractable
  (params (Item :type BPC%20Interactable%20Object%20Reference%20%28by%20ref%29))
  (bind _interactablesinrange (Variables|Default|GetInteractablesInRange))
  (Utilities|Array|RemoveItem _interactablesinrange Item)
  (Utilities|FlowControl|Sequence
    (:then_0
      (if (== (Utilities|Array|Length _interactablesinrange) 1)
        (CallFunction|EndPeriodicChecks)))
    (:then_1
      (if (== Item (Variables|Default|GetActiveInteractable))
        (Variables|Default|SetIsInteracting false)
        (CallFunction|ChooseActiveInteractable)))
    (:then_2
      (EventDispatchers|UnbindEventfromInteractableDestroyed Item (EventDispatchers|CreateEvent :!event RemoveInteractable)))))

(fn ChooseActiveInteractable
  (bind _interactablesinrange (Variables|Default|GetInteractablesInRange))
  (if (not (Variables|Default|GetIsInteracting))
    (switch int (Utilities|Array|Length _interactablesinrange)
      (:Default
        (bind _closestindex (CallFunction|GetClosestInteractable _interactablesinrange (Transformation|GetActorLocation (Components|GetOwner self))))
        (CallFunction|SetActiveInteractable (Utilities|Array|Get(acopy) _interactablesinrange _closestindex)))
      (:0
        (CallFunction|SetActiveInteractable))
      (:1
        (CallFunction|SetActiveInteractable (Utilities|Array|Get(acopy) _interactablesinrange))))))

(fn SetActiveInteractable
  (params (NewActiveInteractable :type BPC%20Interactable%20Object%20Reference))
  (if (!= (Variables|Default|GetActiveInteractable) NewActiveInteractable)
    (Utilities|FlowControl|Sequence
      (:then_0
        ;[1 1 1] Disable previous interactable
        (bind _activeinteractable (Variables|Default|GetActiveInteractable)
          (:then
            (Default|SetasActiveInteractable _activeinteractable false))
          (:else)))
      (:then_1
        ;[1 1 1] Enable new interactable
        (Utilities|IsValid NewActiveInteractable
          (:Is%20Valid
            (Default|SetasActiveInteractable NewActiveInteractable true))))
      (:then_2
        (Variables|Default|SetActiveInteractable NewActiveInteractable)))))

(fn GetClosestInteractable
  (params (Array :type Array%20of%20Actor%20Component%20Object%20References) (ReferencePoint :type Vector))
  (LocalVariables|SetClosestElementIndex -1)
  (for (_array_element _array_index) Array
    (Utilities|IsValid _array_element
      (:Is%20Valid
        (Utilities|FlowControl|Sequence
          (:then_0
            ;[1 1 1] Calculate Current Distance
            (LocalVariables|SetCurrentDistance (Math|Vector|Distance(Vector) (Transformation|GetActorLocation (Components|GetOwner _array_element)) ReferencePoint)))
          (:then_1
            (if (or (< (LocalVariables|GetCurrentDistance) (LocalVariables|GetShortestDistance)) (== (LocalVariables|GetClosestElementIndex) -1))
              (LocalVariables|SetShortestDistance (LocalVariables|GetCurrentDistance))
              (LocalVariables|SetClosestElementIndex _array_index)))))
      (:Is%20Not%20Valid
        (Development|PrintString "Invalid interactable when trying to get the closest one"))))
  (return (LocalVariables|GetClosestElementIndex)))