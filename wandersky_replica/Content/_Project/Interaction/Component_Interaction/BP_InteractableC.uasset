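; BP_InteractableC is an interactable actor with a prompt widget and a sphere that changes to a brick material when interaction completes.
; Its Trigger overlaps report actors entering and leaving range to the BPC_InteractableC component, which owns the interaction logic.
; The component's active-status binding toggles prompt visibility, and its progress events drive the prompt's progress bar, enabled only when a hold time is set.
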(event OnComponentBeginOverlap(Trigger)
  (params (OverlappedComponent :type Primitive%20Component%20Object%20Reference) (OtherActor :type Actor%20Object%20Reference) (OtherComp :type Primitive%20Component%20Object%20Reference) (OtherBodyIndex :type Integer) (bFromSweep :type Boolean) (SweepResult :type Hit%20Result%20Structure%20%28by%20ref%29))
  (Default|PawnEnterRange (Variables|Default|GetBPC_InteractableC) OtherActor))

(event OnComponentEndOverlap(Trigger)
  (params (OverlappedComponent :type Primitive%20Component%20Object%20Reference) (OtherActor :type Actor%20Object%20Reference) (OtherComp :type Primitive%20Component%20Object%20Reference) (OtherBodyIndex :type Integer))
  (Default|PawnExitRange (Variables|Default|GetBPC_InteractableC) OtherActor))

(event InteractionProgress(BPC_InteractableC)
  (params (Percent :type Float%20%28double-precision%29))
  (Default|SetPercent (Variables|Default|GetPromptWidget) Percent))

(event InteractionComplete(BPC_InteractableC)
  (Rendering|Material|SetMaterial (Variables|Default|GetSphere) 0 "/Game/StarterContent/Materials/M_Brick_Clay_Old.M_Brick_Clay_Old"))

(event Custom|EnableWidget
  (params (Active :type Boolean))
  ;[1 1 1] Widget visibility
  (Rendering|SetVisibility (Variables|Default|GetInteractWidget) Active false))

(event EventBeginPlay
  (bind _aswbp_interaction_prompt (Utilities|Casting|CastToWBP_InteractionPrompt (UserInterface|GetWidget (Variables|Default|GetInteractWidget))))
  (Variables|Default|SetPromptWidget _aswbp_interaction_prompt)
  ;[1 1 1] Widget visibility
  (EventDispatchers|BindEventtoChangeActiveStatus (Variables|Default|GetBPC_InteractableC) (delegate Custom|EnableWidget))
  ;[1 1 1] Widget progress bar visibility
  (Default|SetHasProgress (Variables|Default|GetPromptWidget) (> (Variables|/Game/_Project/Interaction/Component_Interaction/BPC_InteractableC.BPC_InteractableC_C|GetHold%20Time (Variables|Default|GetBPC_InteractableC)) 0.0)))

(fn ConstructionScript)