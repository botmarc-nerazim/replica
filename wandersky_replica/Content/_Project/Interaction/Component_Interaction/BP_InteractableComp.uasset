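; Interactable component that lets the third-person character trigger an interacted event by an instant press or a timed hold.
; While the character overlaps the Trigger, it binds to that character's interaction start, ongoing and cancel events, unbinding on exit.
; A positive HoldTime enables hold mode, feeding elapsed time to the prompt widget's progress.
; Completing or canceling a hold resets the state and progress.
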(event Custom|OnInteractionStarted
  (if (Variables|Default|GetRequiresHold)
    (Variables|Default|SetIs%20Interacting true)
    (else
      (Default|CallInteractedEvent))))

(event Custom|OnInteractionOngoing
  (params (Elapsed :type Float%20%28double-precision%29))
  (if (Variables|Default|GetIs%20Interacting)
    (if (>= Elapsed (Variables|Default|GetHoldTime))
      (CallFunction|Reset)
      (Default|CallInteractedEvent)
      (else
        (Default|SetPercent (Variables|Default|GetPromptWidget) (Math|Float|SafeDivide Elapsed (Variables|Default|GetHoldTime)))))))

(event Custom|OnInteractionCanceled
  (CallFunction|Reset))

(event Custom|OnBeginOverlap
  (params (OverlappedComponent :type Primitive%20Component%20Object%20Reference) (OtherActor :type Actor%20Object%20Reference) (OtherComp :type Primitive%20Component%20Object%20Reference) (OtherBodyIndex :type Integer) (bFromSweep :type Boolean) (SweepResult :type Hit%20Result%20Structure%20%28by%20ref%29))
  (bind _asbp_third_person_character (Utilities|Casting|CastToBP_ThirdPersonCharacter OtherActor))
  (EventDispatchers|BindEventtoInteractionStartEvent _asbp_third_person_character (delegate Custom|OnInteractionStarted))
  (EventDispatchers|BindEventtoInteractionOngoingEvent _asbp_third_person_character (delegate Custom|OnInteractionOngoing))
  (EventDispatchers|BindEventtoInteractionCancelEvent _asbp_third_person_character (delegate Custom|OnInteractionCanceled)))

(event Custom|OnEndOverlap
  (params (OverlappedComponent :type Primitive%20Component%20Object%20Reference) (OtherActor :type Actor%20Object%20Reference) (OtherComp :type Primitive%20Component%20Object%20Reference) (OtherBodyIndex :type Integer))
  (bind _asbp_third_person_character (Utilities|Casting|CastToBP_ThirdPersonCharacter OtherActor))
  (EventDispatchers|UnbindEventfromInteractionStartEvent _asbp_third_person_character (delegate Custom|OnInteractionStarted))
  (EventDispatchers|UnbindEventfromInteractionOngoingEvent _asbp_third_person_character (delegate Custom|OnInteractionOngoing))
  (EventDispatchers|UnbindEventfromInteractionCancelEvent _asbp_third_person_character (delegate Custom|OnInteractionCanceled)))

(event EventBeginPlay
  (bind _trigger (Variables|Default|GetTrigger))
  (bind _output_get (Variables|Default|SetRequiresHold (> (Variables|Default|GetHoldTime) 0.0)))
  (Default|SetHasProgress (Variables|Default|GetPromptWidget) _output_get)
  (Collision|BindEventtoOnComponentBeginOverlap _trigger (delegate Custom|OnBeginOverlap))
  (Collision|BindEventtoOnComponentEndOverlap _trigger (delegate Custom|OnEndOverlap)))

(fn Reset
  (Variables|Default|SetIs%20Interacting false)
  (Default|SetPercent (Variables|Default|GetPromptWidget) 0.0))