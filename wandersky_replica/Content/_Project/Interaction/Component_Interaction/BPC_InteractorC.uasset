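; Interactor component that tracks nearby interactables and keeps one active for the owning actor to interact with.
; Add and remove calls maintain the in-range list, starting a looping timer to reselect the closest while several are present.
; Selection pauses during interaction, and switching toggles each interactable's active state.
; Enhanced Input IA_Interact forwards started, ongoing and canceled events to the active interactable.
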(event Custom|Check
  (CallFunction|ChooseActiveInteractable))

(event Custom|StartPeriodicChecks
  (bind _returnvalue (Utilities|Time|SetTimerbyEvent (delegate Custom|Check) 0.2 true 0.2))
  (Variables|Default|SetTimer _returnvalue)
  (Development|PrintString "Start"))

(event Custom|EndPeriodicChecks
  (Utilities|Time|ClearandInvalidateTimerbyHandle (Variables|Default|GetTimer))
  (Development|PrintString "End"))

(event Input|EnhancedActionEvents|EnhancedInputActionIA_Interact
  (params (ActionValue :type Boolean) (ElapsedSeconds :type Float%20%28double-precision%29) (TriggeredSeconds :type Float%20%28double-precision%29) (InputAction :type Input%20Action%20Object%20Reference :default "/Game/ThirdPerson/Input/Actions/IA_Interact.IA_Interact"))
  (bind _activeinteractable (Variables|Default|GetActiveInteractable))
  (:Started
    (Variables|Default|SetIsInteracting true)
    (Utilities|IsValid _activeinteractable
      (:Is%20Valid
        (Default|OnInteractionStarted _activeinteractable))))
  (:Ongoing
    (Utilities|IsValid _activeinteractable
      (:Is%20Valid
        (Default|OnInteractionOngoing _activeinteractable ElapsedSeconds))))
  (:Canceled
    (Variables|Default|SetIsInteracting false)
    (Utilities|IsValid _activeinteractable
      (:Is%20Valid
        (Default|OnInteractionCanceled _activeinteractable)))))

(fn AddInteractable
  (params (NewItem :type BPC%20Interactable%20C%20Object%20Reference%20%28by%20ref%29))
  (bind _interactablesinrange (Variables|Default|GetInteractablesInRange))
  (Utilities|Array|AddUnique _interactablesinrange NewItem)
  (Utilities|FlowControl|Sequence
    (:then_0
      (if (== (Utilities|Array|Length _interactablesinrange) 2)
        (CallFunction|StartPeriodicChecks)))
    (:then_1
      (if (not (Variables|Default|GetIsInteracting))
        (CallFunction|ChooseActiveInteractable)))))

(fn RemoveInteractable
  (params (Item :type BPC%20Interactable%20C%20Object%20Reference%20%28by%20ref%29))
  (bind _interactablesinrange (Variables|Default|GetInteractablesInRange))
  (Utilities|Array|RemoveItem _interactablesinrange Item)
  (Utilities|FlowControl|Sequence
    (:then_0
      (if (== (Utilities|Array|Length _interactablesinrange) 1)
        (CallFunction|EndPeriodicChecks)))
    (:then_1
      (if (== Item (Variables|Default|GetActiveInteractable))
        (Variables|Default|SetIsInteracting false)
        (CallFunction|ChooseActiveInteractable)))))

(fn ChooseActiveInteractable
  (bind _interactablesinrange (Variables|Default|GetInteractablesInRange))
  (if (not (Variables|Default|GetIsInteracting))
    (switch int (Utilities|Array|Length _interactablesinrange)
      (:Default
        (LocalVariables|SetSelfLocation (Transformation|GetActorLocation (Components|GetOwner self)))
        (for _array_element _interactablesinrange
          ;[1 1 1] Is new closest element
          (bind _output_get (LocalVariables|SetCurrentDistance (Math|Vector|Distance(Vector) (LocalVariables|GetSelfLocation) (Transformation|GetActorLocation (Components|GetOwner _array_element)))))
          (if (or (< _output_get (LocalVariables|GetShortestDistance)) (== (LocalVariables|GetShortestDistance) 0.0))
            (LocalVariables|SetShortestDistance _output_get)
            (LocalVariables|SetClosestElement _array_element)))
        (CallFunction|SetActiveInteractable (LocalVariables|GetClosestElement)))
      (:0
        (CallFunction|SetActiveInteractable))
      (:1
        (CallFunction|SetActiveInteractable (Utilities|Array|Get(acopy) _interactablesinrange))))))

(fn SetActiveInteractable
  (params (NewActiveInteractable :type BPC%20Interactable%20C%20Object%20Reference))
  (if (!= (Variables|Default|GetActiveInteractable) NewActiveInteractable)
    (Utilities|FlowControl|Sequence
      (:then_0
        ;[1 1 1] Disable previous interactable
        (Utilities|IsValid (Variables|Default|GetActiveInteractable)
          (:Is%20Valid
            (Default|MakeActive (Variables|Default|GetActiveInteractable) false))))
      (:then_1
        ;[1 1 1] Enable new interactable
        (Utilities|IsValid NewActiveInteractable
          (:Is%20Valid
            (Default|MakeActive NewActiveInteractable true))))
      (:then_2
        (Variables|Default|SetActiveInteractable NewActiveInteractable)))))