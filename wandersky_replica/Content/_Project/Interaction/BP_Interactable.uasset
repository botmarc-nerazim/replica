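; Base-style interactable actor that shows a prompt widget and accepts interact input while the third-person character overlaps its trigger.
; Trigger overlaps toggle the prompt and the actor's own input, resetting progress on exit.
; IA_Interact calls Interacted immediately, or, when HoldTime is above zero, fills the widget's progress until the hold completes and resets on cancel.
; Interacted itself only prints a debug string.
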(event OnComponentBeginOverlap(Trigger)
  (params (OverlappedComponent :type Primitive%20Component%20Object%20Reference) (OtherActor :type Actor%20Object%20Reference) (OtherComp :type Primitive%20Component%20Object%20Reference) (OtherBodyIndex :type Integer) (bFromSweep :type Boolean) (SweepResult :type Hit%20Result%20Structure%20%28by%20ref%29))
  (Utilities|Casting|CastToBP_ThirdPersonCharacter OtherActor)
  (Rendering|SetVisibility (Variables|Default|GetPrompt%20Widget) true false)
  (Input|EnableInput (Game|GetPlayerController 0)))

(event OnComponentEndOverlap(Trigger)
  (params (OverlappedComponent :type Primitive%20Component%20Object%20Reference) (OtherActor :type Actor%20Object%20Reference) (OtherComp :type Primitive%20Component%20Object%20Reference) (OtherBodyIndex :type Integer))
  (Utilities|Casting|CastToBP_ThirdPersonCharacter OtherActor)
  (Rendering|SetVisibility (Variables|Default|GetPrompt%20Widget) false false)
  (Input|DisableInput (Game|GetPlayerController 0))
  (CallFunction|Reset))

(event Input|EnhancedActionEvents|EnhancedInputActionIA_Interact
  (params (ActionValue :type Boolean) (ElapsedSeconds :type Float%20%28double-precision%29) (TriggeredSeconds :type Float%20%28double-precision%29) (InputAction :type Input%20Action%20Object%20Reference :default "/Game/ThirdPerson/Input/Actions/IA_Interact.IA_Interact"))
  (:Started
    (if (Variables|Progress|GetRequiresHold)
      (Variables|Progress|SetIsInteracting true)
      (else
        (CallFunction|Interacted))))
  (:Ongoing
    (if (Variables|Progress|GetIsInteracting)
      (if (>= ElapsedSeconds (Variables|Configuration|GetHoldTime))
        (CallFunction|Reset)
        (CallFunction|Interacted)
        (else
          (Default|SetPercent (Variables|Default|GetTypedWidget) (Math|Float|SafeDivide ElapsedSeconds (Variables|Configuration|GetHoldTime)))))))
  (:Canceled
    (CallFunction|Reset)))

(event EventBeginPlay
  (Variables|Progress|SetRequiresHold (> (Variables|Configuration|GetHoldTime) 0.0))
  (bind _aswbp_interaction_prompt (Utilities|Casting|CastToWBP_InteractionPrompt (UserInterface|GetWidget (Variables|Default|GetPrompt%20Widget))))
  (bind _output_get (Variables|Default|SetTypedWidget _aswbp_interaction_prompt))
  (Default|SetHasProgress _output_get (Variables|Progress|GetRequiresHold)))

(fn ConstructionScript)

(fn Interacted
  (Development|PrintString "Interacted!!!!!!!!!"))

(fn Reset
  (Variables|Progress|SetIsInteracting false)
  (Default|SetPercent (Variables|Default|GetTypedWidget) 0.0))