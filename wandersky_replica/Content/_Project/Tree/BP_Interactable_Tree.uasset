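; BP_Interactable_Tree is an interactable tree that gets planted and grows when the player completes an interaction.
; InteractionComplete from the interactable component marks the tree planted, destroys that component and its widget, and disables the sphere collision, preventing repeat use.
; A float tween with configurable duration and easing scales the static mesh up to GrownScale, then calls the tree-planted event on completion.
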(event InteractionComplete(BPC_Interactable)
  (Utilities|FlowControl|Sequence
    (:then_0
      (Utilities|SetTreeasPlanted))
    (:then_1
      ;[1 1 1] Grow Animation
      (bind _value (|TweenFloat 1.0 (Variables|Default|GetGrownScale) (Variables|Default|GetGrowthDuration) (Variables|Default|GetEase%20Type))
        (:ApplyEasing
          (Transformation|SetWorldScale3D (Variables|Default|GetStaticMesh) (Math|Conversions|ToVector(Float) _value)))
        (:OnComplete
          (Default|CallTreePlantedEvent))))))

(fn ConstructionScript)