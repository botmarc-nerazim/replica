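; GM_CombatMap is the combat map's game mode, tracking how many interactable trees are still waiting to be planted.
; Its construction script scans the level for BP_Interactable_Tree actors, adds each unplanted one to PendingTrees and prints the total.
; OnTreePlanted decrements that counter and prints a completion message at zero, with no further win logic in the file.
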(fn ConstructionScript
  (bind _outactors (Actor|GetAllActorsOfClass "/Game/_Project/Tree/BP_Interactable_Tree.BP_Interactable_Tree_C"))
  (for _array_element _outactors
    (if (not (Variables|/Game/_Project/Tree/BP_Interactable_Tree.BP_Interactable_Tree_C|GetIsPlanted _array_element))
      (Math|Integer|IncrementInt (Variables|Default|GetPendingTrees))))
  (Development|PrintString (Utilities|String|Append "Pending Trees: " (Utilities|String|ToString(Integer) (Variables|Default|GetPendingTrees)))))

(fn OnTreePlanted
  (bind _result (Math|Integer|DecrementInt (Variables|Default|GetPendingTrees))
    (:%20%20
      (if (== _result 0)
        (Development|PrintString "All Trees Planted!!!")))))